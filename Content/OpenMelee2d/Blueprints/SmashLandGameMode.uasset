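; Game mode for a local smash-style fighter of up to four players, adding the in-game UI and spawning each enabled player's character.
; StartMatch creates missing local players and possesses characters spawned at matching PlayerInitialSpawnLocation actors; name lookup always returns KirbyCharacter2.
; LoadLevel saves player setup to the "GameMode" slot before switching levels.
; BeginPlay discards its slot read; LoadLevelData restores setup but is not called here.
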(event Custom|Start%20Match
  (if (Variables|Default|GetEnablePlayer0)
    (bind _out (CallFunction|CharacterNametoOBJ (Variables|Default|GetPlayer0Character)))
    (CallFunction|SpawnCharacter _out))
  (if (Variables|Default|GetEnablePlayer1)
    (bind _out_2 (CallFunction|CharacterNametoOBJ (Variables|Default|GetPlayer1Character)))
    (CallFunction|SpawnCharacter _out_2 1))
  (if (Variables|Default|GetEnablePlayer2)
    (bind _out_3 (CallFunction|CharacterNametoOBJ (Variables|Default|GetPlayer2Character)))
    (CallFunction|SpawnCharacter _out_3 2))
  (if (Variables|Default|GetEnablePlayer3)
    (bind _out_4 (CallFunction|CharacterNametoOBJ (Variables|Default|GetPlayer3Character)))
    (CallFunction|SpawnCharacter _out_4 3)))

(event Custom|LoadLevel
  (params (Name :type String))
  (CallFunction|SaveLevelData)
  (Game|OpenLevel(byName) (Utilities|String|StringToName Name)))

(event EventBeginPlay
  (bind _returnvalue (UserInterface|CreateWidget "/Game/OpenMelee2d/IngameUI/IngameUI.IngameUI_C" (Game|GetPlayerController 0)))
  (UserInterface|Viewport|AddtoViewport _returnvalue 0)
  (SaveGame|LoadGamefromSlot "GameMode"))

(event EventTick
  (params (DeltaSeconds :type Float%20%28single-precision%29)))

(fn ConstructionScript)

(fn CharacterNametoOBJ
  (params (Name :type String))
  (if (Utilities|Enum|Equal(Enum) Name "Kirby")
    _
    (else
      _))
  (LocalVariables|SetCharacter "/Game/OpenMelee2d/Blueprints/KirbyCharacter2.KirbyCharacter2_C")
  (return (LocalVariables|GetCharacter)))

(fn SpawnCharacter
  (params (CharacterObject :type Actor%20Class%20Reference) (Player :type Integer))
  (Utilities|IsValid (Game|GetPlayerController Player)
    (:Is%20Valid
      (Development|PrintString "yes"))
    (:Is%20Not%20Valid
      (Class|GameplayStatics|CreatePlayer -1)))
  (bind _newparam (CallFunction|GetCharacterSpawnPoint Player))
  (bind _returnvalue (Game|SpawnActorfromClass CharacterObject _newparam false 0))
  (bind _ascharacter (Utilities|Casting|CastToCharacter _returnvalue))
  (Pawn|Possess (Game|GetPlayerController Player) _ascharacter))

(fn GetCharacterSpawnPoint
  (params (Player :type Integer))
  (bind _outactors (Actor|GetAllActorsOfClass "/Game/OpenMelee2d/Blueprints/PlayerInitialSpawnLocation.PlayerInitialSpawnLocation_C"))
  (bind _array_element (Utilities|Array|ForEachLoopwithBreak _outactors)
    (:LoopBody
      (bind _asplayer_initial_spawn_location (Utilities|Casting|CastToPlayerInitialSpawnLocation _array_element))
      (if (== (Variables|/Game/OpenMelee2d/Blueprints/PlayerInitialSpawnLocation.PlayerInitialSpawnLocation_C|GetPlayer _asplayer_initial_spawn_location) (Math|Conversions|ToFloat(Integer) Player))
        (return (Transformation|GetActorTransform _asplayer_initial_spawn_location))))))

(fn SaveLevelData
  (bind _returnvalue (SaveGame|CreateSaveGameObject "/Game/OpenMelee2d/Blueprints/GameModeSave.GameModeSave_C"))
  (bind _asgame_mode_save (Utilities|Casting|CastToGameModeSave _returnvalue))
  (Variables|/Game/OpenMelee2d/Blueprints/GameModeSave.GameModeSave_C|SetEnablePlayer0 _asgame_mode_save (Variables|Default|GetEnablePlayer0))
  (Variables|/Game/OpenMelee2d/Blueprints/GameModeSave.GameModeSave_C|SetEnablePlayer1 _asgame_mode_save (Variables|Default|GetEnablePlayer1))
  (Variables|/Game/OpenMelee2d/Blueprints/GameModeSave.GameModeSave_C|SetEnablePlayer2 _asgame_mode_save (Variables|Default|GetEnablePlayer2))
  (Variables|/Game/OpenMelee2d/Blueprints/GameModeSave.GameModeSave_C|SetEnablePlayer3 _asgame_mode_save (Variables|Default|GetEnablePlayer3))
  (Variables|/Game/OpenMelee2d/Blueprints/GameModeSave.GameModeSave_C|SetPlayer0Character _asgame_mode_save (Variables|Default|GetPlayer0Character))
  (Variables|/Game/OpenMelee2d/Blueprints/GameModeSave.GameModeSave_C|SetPlayer1Character _asgame_mode_save (Variables|Default|GetPlayer1Character))
  (Variables|/Game/OpenMelee2d/Blueprints/GameModeSave.GameModeSave_C|SetPlayer2Character _asgame_mode_save (Variables|Default|GetPlayer2Character))
  (Variables|/Game/OpenMelee2d/Blueprints/GameModeSave.GameModeSave_C|SetPlayer3Character _asgame_mode_save (Variables|Default|GetPlayer3Character))
  (SaveGame|SaveGametoSlot _asgame_mode_save "GameMode"))

(fn LoadLevelData
  (bind _returnvalue (SaveGame|LoadGamefromSlot "GameMode"))
  (bind _asgame_mode_save (Utilities|Casting|CastToGameModeSave _returnvalue))
  (Variables|Default|SetEnablePlayer0 (Variables|/Game/OpenMelee2d/Blueprints/GameModeSave.GameModeSave_C|GetEnablePlayer0 _asgame_mode_save))
  (Variables|Default|SetEnablePlayer1 (Variables|/Game/OpenMelee2d/Blueprints/GameModeSave.GameModeSave_C|GetEnablePlayer1 _asgame_mode_save))
  (Variables|Default|SetEnablePlayer2 (Variables|/Game/OpenMelee2d/Blueprints/GameModeSave.GameModeSave_C|GetEnablePlayer2 _asgame_mode_save))
  (Variables|Default|SetEnablePlayer3 (Variables|/Game/OpenMelee2d/Blueprints/GameModeSave.GameModeSave_C|GetEnablePlayer3 _asgame_mode_save))
  (Variables|Default|SetPlayer0Character (Variables|/Game/OpenMelee2d/Blueprints/GameModeSave.GameModeSave_C|GetPlayer0Character _asgame_mode_save))
  (Variables|Default|SetPlayer1Character (Variables|/Game/OpenMelee2d/Blueprints/GameModeSave.GameModeSave_C|GetPlayer1Character _asgame_mode_save))
  (bind _output_get (Variables|Default|SetPlayer2Character (Variables|/Game/OpenMelee2d/Blueprints/GameModeSave.GameModeSave_C|GetPlayer2Character _asgame_mode_save)))
  (Variables|Default|SetPlayer3Character (Variables|/Game/OpenMelee2d/Blueprints/GameModeSave.GameModeSave_C|GetPlayer3Character _asgame_mode_save))
  (Development|PrintString _output_get))