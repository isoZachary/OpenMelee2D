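; ControllerToPlayer is an interface-style set of stub functions for exchanging combat state between controller and player in OpenMelee2d, a 2D fighting game.
; It declares queries for the current attack's knockback, direction and damage, plus hit stun, percentage and a damage sprite.
; It also declares a CleanAttack call returning a float.
; All bodies return only defaults, so the actual logic lives outside this file.
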(fn GetDamageSprite
  (return 0))

(fn GetCurrentAtackKnockBack
  (return 0.0))

(fn GetCurrentAtackDirection
  (return ""))

(fn GetCurrentAtackDamage
  (return 0.0))

(fn GetHitStun
  (return false))

(fn GetPercentage
  (return 0.0))

(fn CleanAttack
  (return 0.0))