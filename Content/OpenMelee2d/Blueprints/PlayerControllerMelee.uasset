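; Player controller for a 2D Melee-style fighter, handling player death, respawn and access to pawn combat state.
; Getters forward damage, attack, hitstun and percentage queries to the pawn through messages; SetHitStun is empty.
; KillPlayer spawns an explosion referencing the controller and destroys the pawn.
; RevivePlayer matches player index to a respawn point, falling back to unused ones without a loop break, then spawns and possesses a movement-disabled, reviving Kirby.
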(event EventBeginPlay)

(event EventTick
  (params (DeltaSeconds :type Float%20%28single-precision%29)))

(fn ConstructionScript)

(fn GetDamageSprite
  (bind _collisoinsprite (Class|ControllertoPlayer|GetDamageSprite(Message) (Pawn|GetControlledPawn)))
  (return _collisoinsprite))

(fn SetHitStun
  (params (%20  :type Boolean :default false)))

(fn GetCurrentAttackDirection
  (bind _direction (Class|ControllertoPlayer|GetCurrentAtackDirection(Message) (Pawn|GetControlledPawn)))
  (return _direction))

(fn GetCurrentAttackKnockback
  (bind _kb (Class|ControllertoPlayer|GetCurrentAtackKnockBack(Message) (Pawn|GetControlledPawn)))
  (return _kb))

(fn GetCurrentAttackDamage
  (bind _damage (Class|ControllertoPlayer|GetCurrentAtackDamage(Message) (Pawn|GetControlledPawn)))
  (Development|PrintString (Utilities|String|Append (Utilities|String|ToString(Float) _damage) "sa"))
  (return _damage))

(fn GetHitStun
  (bind _newparam (Class|ControllertoPlayer|GetHitStun(Message) (Pawn|GetControlledPawn)))
  (return _newparam))

(fn GetPercentage
  (bind _newparam (Class|ControllertoPlayer|GetPercentage(Message) (Pawn|GetControlledPawn)))
  (Development|PrintString (Utilities|String|Append (Utilities|String|ToString(Float) _newparam) "ffdsfsddsf"))
  (return _newparam))

(fn CleanAttack
  (Class|ControllertoPlayer|CleanAttack(Message) (Pawn|GetControlledPawn)))

(fn KillPlayer
  (params (Right :type Boolean) (Left :type Boolean) (Top :type Boolean) (Bottom :type Boolean) (Location :type Vector :default "0, 0, 0"))
  (bind _returnvalue (Pawn|GetControlledPawn))
  (bind _ascharacter (Utilities|Casting|CastToCharacter _returnvalue))
  (bind _returnvalue_2 (Game|SpawnActorfromClass "/Game/OpenMelee2d/Misc/BlastZone/Explosion.Explosion_C" (Math|Transform|MakeTransform Location) false 0))
  (Variables|/Game/OpenMelee2d/Misc/BlastZone/Explosion.Explosion_C|SetPlayerControllerT _returnvalue_2 self)
  (Actor|DestroyActor _returnvalue))

(fn RevivePlayer
  (bind _outactors (Actor|GetAllActorsOfClass "/Game/OpenMelee2d/Misc/BlastZone/PlayerReSpawnLocation.PlayerReSpawnLocation_C"))
  ;[1 1 1] Comment
  (if (== (Game|GetPlayerController 0) self)
    ;;[1 1 1] Comment
    (bind _array_element (Utilities|Array|ForEachLoopwithBreak _outactors)
      (:LoopBody
        (if (== (Variables|/Game/OpenMelee2d/Misc/BlastZone/PlayerReSpawnLocation.PlayerReSpawnLocation_C|GetNumber _array_element) 0)
          (LocalVariables|SetReviveTransform (Transformation|GetActorTransform _array_element))
          (LocalVariables|SetRevivePlatform _array_element)
          (if (Variables|/Game/OpenMelee2d/Misc/BlastZone/PlayerReSpawnLocation.PlayerReSpawnLocation_C|GetIsUsed (LocalVariables|GetRevivePlatform)) :!label _label
            (bind _array_element_2 (Utilities|Array|ForEachLoopwithBreak _outactors)
              (:LoopBody
                (if (not (Variables|/Game/OpenMelee2d/Misc/BlastZone/PlayerReSpawnLocation.PlayerReSpawnLocation_C|GetIsUsed _array_element_2))
                  (LocalVariables|SetReviveTransform (Transformation|GetActorTransform _array_element_2))
                  ;[1 1 1] Comment
                  (bind _returnvalue (Game|SpawnActorfromClass "/Game/OpenMelee2d/Blueprints/KirbyCharacter2.KirbyCharacter2_C" (LocalVariables|GetReviveTransform) false 0 :!label _label_2))
                  (Variables|/Game/OpenMelee2d/Blueprints/KirbyCharacter2.KirbyCharacter2_C|SetIsReviving _returnvalue true)
                  (Pawn|Possess _returnvalue)
                  (Pawn|Components|CharacterMovement|SetMovementMode _returnvalue "MOVE_None" 0))))
            (else
              (goto _label_2))))))
    (elif (== (Game|GetPlayerController 1) self)
      ;;[1 1 1] Comment
      (bind _array_element_3 (Utilities|Array|ForEachLoopwithBreak _outactors)
        (:LoopBody
          (if (== (Variables|/Game/OpenMelee2d/Misc/BlastZone/PlayerReSpawnLocation.PlayerReSpawnLocation_C|GetNumber _array_element_3) 1)
            (LocalVariables|SetReviveTransform (Transformation|GetActorTransform _array_element_3))
            (LocalVariables|SetRevivePlatform _array_element_3)
            (goto _label))))
      (elif (== (Game|GetPlayerController 2) self)
        ;;[1 1 1] Comment
        (bind _array_element_4 (Utilities|Array|ForEachLoopwithBreak _outactors)
          (:LoopBody
            (if (== (Variables|/Game/OpenMelee2d/Misc/BlastZone/PlayerReSpawnLocation.PlayerReSpawnLocation_C|GetNumber _array_element_4) 2)
              (LocalVariables|SetReviveTransform (Transformation|GetActorTransform _array_element_4))
              (LocalVariables|SetRevivePlatform _array_element_4)
              (goto _label))))
        (elif (== (Game|GetPlayerController 3) self)
          ;;[1 1 1] Comment
          (bind _array_element_5 (Utilities|Array|ForEachLoopwithBreak _outactors)
            (:LoopBody
              (if (== (Variables|/Game/OpenMelee2d/Misc/BlastZone/PlayerReSpawnLocation.PlayerReSpawnLocation_C|GetNumber _array_element_5) 3)
                (LocalVariables|SetReviveTransform (Transformation|GetActorTransform _array_element_5))
                (LocalVariables|SetRevivePlatform _array_element_5)
                (goto _label)))))))))